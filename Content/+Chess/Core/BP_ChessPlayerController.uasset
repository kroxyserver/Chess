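; Player controller for the chess game that manages the player's UI and move sound.
; BeginPlay adds the main player HUD and binds to the piece-moved event, with a move-effect handler that plays a 2D sound.
; Spawn events open a high Z-order pawn promotion widget for the given board and pawn, or replace the HUD with a game-over screen and switch input to UI-only.
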(event Custom|OnPieceMovedFX
  (params (bIsWhite :type Boolean))
  (Audio|PlaySound2D "/Game/Assets/Sounds/SW_ChessPiece_Move.SW_ChessPiece_Move" 1.0 1.0 0.0 0 0))

(event EventBeginPlay
  (bind _returnvalue (UserInterface|CreateWidget "/Game/+Chess/UI/Game/WBP_ChessPlayerUI.WBP_ChessPlayerUI_C" self))
  (bind _output_get (Variables|Default|SetPlayerUI _returnvalue))
  (UserInterface|Viewport|AddtoViewport _output_get 0)
  (EventDispatchers|AssignOnPieceMoved (EventDispatchers|CreateEvent :!event Custom|OnPieceMovedFX)))

(event EventSpawnGameOverUI
  (params (GameState :type EChessGameState%20Enum :default "Ongoing") (bIsWhiteTurn :type Boolean))
  (bind _playerui (Variables|Default|GetPlayerUI)
    (:then
      (Widget|RemovefromParent _playerui)
      (bind _returnvalue (UserInterface|CreateWidget "/Game/+Chess/UI/Game/WBP_GameOverUI.WBP_GameOverUI_C" self GameState bIsWhiteTurn))
      (UserInterface|Viewport|AddtoViewport _returnvalue 0)
      (Input|SetInputModeUIOnly self _returnvalue "DoNotLock" false))
    (:else)))

(event EventSpawnPawnPromotionUI
  (params (ChessBoard :type Chess%20Board%20Object%20Reference) (PawnToPromote :type Chess%20Piece%20Object%20Reference))
  (bind _returnvalue (UserInterface|CreateWidget "/Game/+Chess/UI/Game/WBP_PawnPromotionUI.WBP_PawnPromotionUI_C" self ChessBoard PawnToPromote))
  (UserInterface|Viewport|AddtoViewport _returnvalue 99))

(fn ConstructionScript)