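; BP_ChessPlayer is the chess player Blueprint that swings its spring arm between the white and black views of the board.
; SwitchPlayerView plays a timeline toward black or reverses it toward white, lerping the arm through a half turn at a fixed downward tilt.
; BeginPlay scales the timeline's play rate to set the swing speed.
; An unconnected instant-snap rotation remains in the graph.
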(event EventBeginPlay
  (Components|Timeline|SetPlayRate (Variables|Default|GetTL_SwitchPlayerView) (/ 1.0 1.2)))

(event EventSwitchPlayerView
  (params (bToWhite :type Boolean))
  (if (not bToWhite)
    (bind _alpha (Timeline|TL_SwitchPlayerView Play)
      (:Update
        (Transformation|SetRelativeRotation (Variables|Default|GetSpringArmComponent) (Math|Rotator|Lerp(Rotator) "-65.000000,0.000000,0.000000" "-65.000000,180.000000,0.000000" _alpha true) false false)))
    (else
      (Timeline|TL_SwitchPlayerView Reverse))))

(fn ConstructionScript)