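; BP_ChessTile is a chess board tile Blueprint with a sphere that is meant to indicate which side attacks the tile.
; Disconnected EventGraph logic sets the sphere's visibility from the white and black attack flags in ChessTileInfo.
; It then picks a bright, dark or combined material, with the both-sides case applied last to override the others.
; No event triggers this logic, and the construction script is empty.
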(fn ConstructionScript)